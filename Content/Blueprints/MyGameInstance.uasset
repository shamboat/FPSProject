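; Game instance Blueprint that holds the shared ammo count and relays text messages for the UI.
; AddAmmo increases the count, while SubtractAmmo decreases it and clamps the result at zero.
; DisplayUIMessage and DisplayUILookAtMessage pass their text on through separate UI calls, one for general messages and one for look-at messages.
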(event `AddAmmo`
  (params (IncomingAmmo :type Integer))
  (set `self.Ammo` (+ IncomingAmmo (`self.Ammo`))))

(event `SubtractAmmo`
  (params (AmmoToBeRemoved :type Integer))
  (bind _returnvalue (- (`self.Ammo`) AmmoToBeRemoved))
  (if (< _returnvalue 0)
    (set `self.Ammo` 0)
    (else
      (set `self.Ammo` _returnvalue))))

(event `DisplayUIMessage`
  (params (IncomingText :type Text))
  (`self.UIDisplayMessage` IncomingText))

(event `DisplayUILookAtMessage`
  (params (IncomingText :type Text))
  (`self.UIDisplayLookAtMessage` IncomingText))
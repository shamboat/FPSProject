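; BP_Button is an interactable button that relays interaction to a target object and returns messages for Interact and LookAt.
; Interacting plays a shutter sound and starts a timeline that lerps the button's dynamic material from pink to green.
; On every timeline update, it calls the target through InteractableInterface, or plays a failure sound if the target lacks that interface.
; Interact always reports DidInteract as false.
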(event `self.ReceiveBeginPlay`
  (bind _returnvalue (`KismetMaterialLibrary.CreateDynamicMaterialInstance` "/Game/Material/M_Button.M_Button"))
  (bind _output_get (set `self.ButtonMaterial` _returnvalue))
  (`PrimitiveComponent.SetMaterial` (`self.Button`) 0 _output_get)
  (`MaterialInstanceDynamic.SetVectorParameterValue` (`self.ButtonMaterial`) "ButtonColor" (struct :`R` 1.0 :`G` 0.160784 :`B` 0.933333 :`A` 1.0)))

(event `PushButton`
  (bind _targetinteractable (`self.TargetInteractable`))
  ;[1 1 1] Play a sound
  (`GameplayStatics.PlaySound2D` "/Engine/VREditor/Sounds/UI/Camera_Shutter.Camera_Shutter" 1.0 1.0 0.0 null null)
  (bind (_direction _newtrack_0) (`Timeline|ButtonColor` :!via `PlayFromStart`)
    (:`Update`
      (`MaterialInstanceDynamic.SetVectorParameterValue` (`self.ButtonMaterial`) "ButtonColor" (`KismetMathLibrary.LinearColorLerp` (struct :`R` 1.0 :`G` 0.160784 :`B` 0.933333 :`A` 1.0) (struct :`G` 1.0 :`B` 0.174587 :`A` 1.0) _newtrack_0))
      ;[1 1 1] Is the target object interactable?
      (if (`KismetSystemLibrary.DoesImplementInterface` _targetinteractable "/Game/Blueprints/InteractableInterface.InteractableInterface_C")
        ;[1 1 1] Interact with target object
        (message `/Game/Blueprints/InteractableInterface.Interact` _targetinteractable)
        (else
          ;[1 1 1] Failed interaction
          (`GameplayStatics.PlaySound2D` "/Engine/EditorSounds/Notifications/CompileFailed.CompileFailed" 1.0 1.0 0.0 null null))))))

(fn `Interact`
  (returns (DidInteract :type Boolean) (Message :type Text))
  (`self.PushButton`)
  (return false (`self.InteractionMessage`)))

(fn `LookAt`
  (returns (Message :type Text))
  (return (`self.LookAtMessage`)))

(fn `UserConstructionScript`)
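; Wall lamp that the player can switch on and off through Interact, glowing green-cyan when lit.
; BeginPlay gives the Lamp mesh a dynamic material instance with LampColor starting at black.
; Interact calls ToggleLamp, where a FlipFlop plays or reverses the LampPower timeline to fade that color parameter.
; Interact always reports DidInteract as false, and both it and LookAt return empty text.
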(event `self.ReceiveBeginPlay`
  ;[1 1 1] Material setup
  (bind _returnvalue (`KismetMaterialLibrary.CreateDynamicMaterialInstance` "/Game/Material/MI_WallLAmp.MI_WallLAmp"))
  (bind _output_get (set `self.LampMaterial` _returnvalue))
  (`PrimitiveComponent.SetMaterial` (`self.Lamp`) 0 _output_get)
  (`MaterialInstanceDynamic.SetVectorParameterValue` :`self` (`self.LampMaterial`) :`ParameterName` "LampColor"))

(event `ToggleLamp`
  (`/Engine/EditorBlueprintResources/StandardMacros.FlipFlop`
    (:`A`
      (bind (_direction _power) (`Timeline|LampPower` :!label _label)
        (:`Update`
          (`MaterialInstanceDynamic.SetVectorParameterValue` (`self.LampMaterial`) "LampColor" (`KismetMathLibrary.LinearColorLerp` (struct) (struct :`G` 1.0 :`B` 0.557249 :`A` 1.0) _power)))))
    (:`B`
      (goto _label :!via `Reverse`))))

(fn `Interact`
  (returns (DidInteract :type Boolean) (Message :type Text))
  (`self.ToggleLamp`)
  (return false ""))

(fn `LookAt`
  (returns (Message :type Text))
  (return ""))

(fn `UserConstructionScript`)
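; Door actor Blueprint that the player can look at and interact with to open or close it.
; On BeginPlay it casts the Door mesh's anim instance to DoorAnimation and caches it as DoorAnimator.
; Interact calls ToggleDoor, where a FlipFlop alternates SetOpen and SetClosed on the animation Blueprint, then returns false with an empty message.
; LookAt returns the stored LookAtMessage.
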(event `self.ReceiveBeginPlay`
  ;[1 1 1] Animation blueprint linking
  (bind _asdoor_animation (cast `/Game/Assets/Door/DoorAnimation` (`SkeletalMeshComponent.GetAnimInstance` (`self.Door`)))) ; Store anim blueprints to memory
  (set `self.DoorAnimator` _asdoor_animation) ; Store as a variable
)

(event `ToggleDoor`
  (bind _dooranimator (`self.DoorAnimator`))
  ;[1 1 1] Test door opening
  (`/Engine/EditorBlueprintResources/StandardMacros.FlipFlop`
    (:`A`
      (`/Game/Assets/Door/DoorAnimation.SetOpen` _dooranimator))
    (:`B`
      (`/Game/Assets/Door/DoorAnimation.SetClosed` _dooranimator))))

(fn `Interact`
  (returns (DidInteract :type Boolean) (Message :type Text))
  (`self.ToggleDoor`)
  (return false ""))

(fn `LookAt`
  (returns (Message :type Text))
  (return (`self.LookAtMessage`)))

(fn `UserConstructionScript`)